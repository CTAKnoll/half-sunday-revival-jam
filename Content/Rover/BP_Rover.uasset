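; BP_Rover is a six-wheeled rover that uses raycast hover suspension to push its physics body off the ground.
; Every Tick, SuspensionCast runs a downward Visibility line trace from each wheel component, drawn for debugging.
; On a hit, it applies an upward force to the Collider at that wheel, growing linearly as the hit gets closer and scaled by HoverMultiplier, with no damping term.
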(event `self.ReceiveTick`
  (params (DeltaSeconds :type "Float (single-precision)"))
  (for _array_element (`|MakeArray` (`self.FL_Wheel`) (`self.FR_Wheel`) (`self.ML_Wheel`) (`self.MR_Wheel`) (`self.BL_Wheel`) (`self.BR_Wheel`))
    (`self.SuspensionCast` _array_element)))

(fn `SuspensionCast`
  (params (WheelComponent :type "SceneComponent Object Reference"))
  (bind _returnvalue (`SceneComponent.K2_GetComponentLocation` WheelComponent))
  (bind _outhit (`KismetSystemLibrary.LineTraceSingle` :`Start` _returnvalue :`End` (+ _returnvalue (* (`self.CastDistance`) (`KismetMathLibrary.Vector_Down`))) :`TraceChannel` "TraceTypeQuery1" :`DrawDebugType` "ForOneFrame"))
  (bind (_bblockinghit _binitialoverlap _time _distance _location _impactpoint _normal _impactnormal _physmat _hitactor _hitcomponent _hitbonename _bonename _hititem _elementindex _faceindex _tracestart _traceend) (`GameplayStatics.BreakHitResult` _outhit))
  (if _bblockinghit
    (`PrimitiveComponent.AddForceAtLocation` (`self.Collider`) (* (- 1.0 (`KismetMathLibrary.NormalizeToRange` _distance 0.0 (`self.CastDistance`))) (`KismetMathLibrary.GetDirectionUnitVector` _traceend _tracestart) (`self.HoverMultiplier`)) (`SceneComponent.K2_GetComponentLocation` (`local.WheelComponent`)) "None")))

(fn `UserConstructionScript`)